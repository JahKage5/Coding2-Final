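; Game mode that saves and loads per-level state and player stats through SaveGame objects.
; On BeginPlay it loads or creates a level save keyed by level name, calling LoadStateMessage on each altered actor.
; It also loads or creates a shared "PlayerSave" slot, restoring only the character's Stamina.
; Separate events write both saves; coin, door and held-item restore logic is disconnected.
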(event Custom|Load%20Player%20Stats
  (bind _returnvalue (SaveGame|DoesSaveGameExist "PlayerSave"))
  (if _returnvalue
    (bind _returnvalue_2 (SaveGame|LoadGamefromSlot "PlayerSave"))
    (bind _assg_player_stats (Utilities|Casting|CastToSG_PlayerStats _returnvalue_2))
    (Variables|Default|SetSG_PlayerStats _assg_player_stats)
    (bind _asbp_third_person_character (Utilities|Casting|CastToBP_ThirdPersonCharacter (Game|GetPlayerCharacter 0)))
    (Variables|/Game/ThirdPerson/Blueprints/BP_ThirdPersonCharacter.BP_ThirdPersonCharacter_C|SetStamina _asbp_third_person_character (Variables|/Game/Blueprints/SavingLoading/SG_PlayerStats.SG_PlayerStats_C|GetStamina (Variables|Default|GetSG_PlayerStats))) ; The Player's Stamina
    (else
      (bind _returnvalue_3 (SaveGame|CreateSaveGameObject "/Game/Blueprints/SavingLoading/SG_PlayerStats.SG_PlayerStats_C"))
      (Variables|Default|SetSG_PlayerStats _returnvalue_3) ; set this variable so that the \nPlayer can edit these values
    )))

(event Custom|Save%20Player%20Stats
  (Game|GetCurrentLevelName true)
  (bind _returnvalue (SaveGame|SaveGametoSlot (Variables|Default|GetSG_PlayerStats) "PlayerSave"))
  (if _returnvalue
    (Development|PrintText "Player Stats Written to Save Game File" true true "(R=0.321655,G=1.000000,B=0.013734,A=1.000000)" 5.0)
    (else
      (Development|PrintText "Player Stats Could Not be Written to Save Game File" true true "(R=1.000000,G=0.000528,B=0.043477,A=1.000000)" 5.0))))

(event Custom|SaveLevelStateToFile
  (bind _returnvalue (Game|GetCurrentLevelName true))
  (bind _returnvalue_2 (SaveGame|SaveGametoSlot (Variables|Default|GetSG_LevelStatee) _returnvalue))
  (if _returnvalue_2
    (Development|PrintText "Level State Saved" true true "(R=0.321655,G=1.000000,B=0.013734,A=1.000000)" 5.0)
    (else
      (Development|PrintText "Level State Failed To Save" true true "(R=1.000000,G=0.000000,B=0.030010,A=1.000000)" 5.0))))

(event Custom|Load%20Level%20State%20From%20File
  (bind _returnvalue (Game|GetCurrentLevelName true))
  (bind _returnvalue_2 (SaveGame|DoesSaveGameExist _returnvalue))
  (if _returnvalue_2
    (bind _returnvalue_3 (SaveGame|LoadGamefromSlot _returnvalue))
    (bind _assg_level_statee (Utilities|Casting|CastToSG_LevelStatee _returnvalue_3)
      (:then
        (Variables|Default|SetSG_LevelStatee _assg_level_statee)
        (Development|PrintString "Loaded existing level state")
        (for _array_element (Variables|/Game/Blueprints/SavingLoading/SG_LevelStatee.SG_LevelStatee_C|GetAlteredActors (Variables|Default|GetSG_LevelStatee))
          (Class|BPILevelActorSaveable|LoadState(Message) _array_element) ; maybe need an isValid check before this
          (Development|PrintString "called load state from GMsavlod2")))
      (:CastFailed
        (Development|PrintString "cast failed")))
    (else
      (bind _returnvalue_4 (SaveGame|CreateSaveGameObject "/Game/Blueprints/SavingLoading/SG_LevelStatee.SG_LevelStatee_C"))
      (Variables|Default|SetSG_LevelStatee _returnvalue_4)
      (Development|PrintString "new save game for level state has been created"))))

(event EventBeginPlay
  (CallFunction|LoadLevelStatefromFile)
  (CallFunction|LoadPlayerStats))

(fn ConstructionScript)