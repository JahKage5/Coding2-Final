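; BP_SecurityCamera is a sweeping security camera that flags the player as detected in BP_GameInstance when its box is overlapped.
; A self-reversing timeline swings the camera yaw back and forth until an overlap stops it and swaps the StatusLED decal material.
; Each tick, a very short debug-drawn trace from the scene capture positions that decal at the impact point.
; OnSeeTarget only prints debug messages.
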(event OnComponentBeginOverlap(Box)
  (params (OverlappedComponent :type Primitive%20Component%20Object%20Reference) (OtherActor :type Actor%20Object%20Reference) (OtherComp :type Primitive%20Component%20Object%20Reference) (OtherBodyIndex :type Integer) (bFromSweep :type Boolean) (SweepResult :type Hit%20Result%20Structure%20%28by%20ref%29))
  (Variables|/Game/Blueprints/BP_GameInstance.BP_GameInstance_C|SetIsPlayerDetected (Variables|Default|GetGameInstanceRef) true)
  (Rendering|Components|Decal|SetDecalMaterial (Variables|Default|GetStatusLED) "/Game/Materials/DecalMaterials/M_CameraProjection_Inst.M_CameraProjection_Inst")
  (CallFunction|BlockTimeline))

(event Custom|Block%20Timeline
  (bind _camera (Variables|Default|GetCamera))
  (bind _relativerotation (Variables|/Script/Engine.SceneComponent|GetRelativeRotation _camera))
  (bind _moving_value (Timeline|Timeline Stop)
    (:Update
      (Transformation|SetRelativeRotation (Variables|Default|GetCamera) (Math|Rotator|Lerp(Rotator) (Math|Rotator|MakeRotator (.roll _relativerotation) (.pitch _relativerotation) -45.0) (Math|Rotator|MakeRotator (.roll _relativerotation) (.pitch _relativerotation) 45.0) _moving_value) false false))
    (:Finished
      (if (Variables|Default|GetItRestarts?)
        (Variables|Default|SetItRestarts? false)
        (Timeline|Timeline Play)
        (else
          (Variables|Default|SetItRestarts? true)
          (Timeline|Timeline Reverse))))))

(event EventBeginPlay
  (bind _camera (Variables|Default|GetCamera))
  (bind _relativerotation (Variables|/Script/Engine.SceneComponent|GetRelativeRotation _camera))
  (bind _asbp_game_instance (Utilities|Casting|CastToBP_GameInstance (Game|GetGameInstance)))
  (Variables|Default|SetGameInstanceRef _asbp_game_instance)
  (bind _moving_value (Timeline|Timeline Play)
    (:Update
      (Transformation|SetRelativeRotation (Variables|Default|GetCamera) (Math|Rotator|Lerp(Rotator) (Math|Rotator|MakeRotator (.roll _relativerotation) (.pitch _relativerotation) -45.0) (Math|Rotator|MakeRotator (.roll _relativerotation) (.pitch _relativerotation) 45.0) _moving_value) false false))
    (:Finished
      (if (Variables|Default|GetItRestarts?)
        (Variables|Default|SetItRestarts? false)
        (Timeline|Timeline Play)
        (else
          (Variables|Default|SetItRestarts? true)
          (Timeline|Timeline Reverse))))))

(event EventTick
  (params (DeltaSeconds :type Float%20%28single-precision%29))
  (bind _scenecapturecomponent2d (Variables|Default|GetSceneCaptureComponent2D))
  (bind _returnvalue (Transformation|GetWorldLocation _scenecapturecomponent2d))
  (bind _outhit (Collision|LineTraceByChannel _returnvalue (+ _returnvalue (Math|Vector|GetForwardVector (Variables|Default|GetSceneCaptureComponent2D))) "TraceTypeQuery1" false 0 "ForOneFrame"))
  (Transformation|SetWorldLocationAndRotation (Variables|Default|GetStatusLED) (.ImpactPoint (Collision|BreakHitResult _outhit)) (Math|Conversions|RotationFromXVector (.ImpactNormal (Collision|BreakHitResult _outhit))) false false))

(fn ConstructionScript)

(fn OnSeeTarget
  (Development|PrintString "I see the enemy!")
  (switch Utilities|FlowControl|Switch|SwitchonE_AIState "NewEnumerator3" ; if we're attacking, don't switch\nto investigating
    (:NewEnumerator3
      (Development|PrintText "That's not our enemy!") ; doesn't change state if detecting a friendly\n(a non-player)
    )))