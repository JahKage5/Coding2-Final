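; BP_CamDoorTrigger is a trigger that opens a linked door when the third-person player character steps into it.
; Overlapping its sphere plays a pressure plate sound and calls OpenDoor on the Target, passing the player as the new view target.
; It then adds the door to the GM_SaveLod2 game mode's level-state list of altered actors, without duplicates.
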(event OnComponentBeginOverlap(Sphere1)
  (params (OverlappedComponent :type Primitive%20Component%20Object%20Reference) (OtherActor :type Actor%20Object%20Reference) (OtherComp :type Primitive%20Component%20Object%20Reference) (OtherBodyIndex :type Integer) (bFromSweep :type Boolean) (SweepResult :type Hit%20Result%20Structure%20%28by%20ref%29))
  (Utilities|Casting|CastToBP_ThirdPersonCharacter OtherActor)
  (Audio|PlaySoundatLocation "/Game/Audio/PressurePlateCue.PressurePlateCue" (Transformation|GetActorLocation) "0, 0, 0" 1.0 1.0 0.0 0 0 0 0)
  (Default|OpenDoor (Variables|Default|GetTarget) OtherActor) ; new view target is the player
  (bind _asgm_save_lod_2 (Utilities|Casting|CastToGM_SaveLod2 (Game|GetGameMode)))
  (Utilities|Array|AddUnique (Variables|/Game/Blueprints/SavingLoading/SG_LevelStatee.SG_LevelStatee_C|GetAlteredActors (Variables|/Game/Blueprints/SavingLoading/GM_SaveLod2.GM_SaveLod2_C|GetSG_LevelStatee _asgm_save_lod_2)) (Variables|Default|GetTarget)))

(event EventBeginPlay)

(event Collision|EventActorBeginOverlap
  (params (OtherActor :type Actor%20Object%20Reference)))

(event EventTick
  (params (DeltaSeconds :type Float%20%28single-precision%29)))

(fn ConstructionScript)