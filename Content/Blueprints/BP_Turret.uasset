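; BP_Turret is a turret that turns to face and shoots at the third-person player character when its PawnSensing component sees it.
; On a sighting it snaps its rotation toward the character, waits through a short delay, plays a cannon sound and spawns a bullet actor at its Arrow component's transform.
; The aim is set before the delay, so the shot follows the turret's facing at fire time.
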(event OnSeePawn(PawnSensing)
  (params (Pawn :type Pawn%20Object%20Reference))
  (Utilities|Casting|CastToBP_ThirdPersonCharacter Pawn)
  (Transformation|SetActorRotation (Math|Rotator|FindLookatRotation (Transformation|GetActorLocation) (Transformation|GetActorLocation Pawn)))
  (Utilities|FlowControl|Delay 2.0)
  (Audio|PlaySoundatLocation "/Game/Audio/CannonBeamCue.CannonBeamCue" (Transformation|GetActorLocation) "0, 0, 0" 1.0 1.0 0.0 0 0 0 0)
  (Game|SpawnActorfromClass "/Game/Blueprints/BP_Bullet1.BP_Bullet1_C" (Transformation|GetWorldTransform (Variables|Default|GetArrow)) "Undefined" "MultiplyWithRoot" 0 0))

(fn ConstructionScript)